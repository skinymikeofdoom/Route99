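; BP_Obsicle is a physics-simulated obstacle actor with a randomized appearance.
; Its construction script picks a random mesh and, independently, a random slot-0 material from two arrays, so the look re-rolls whenever construction reruns.
; It also enables physics on the static mesh and greatly raises its mass scale to make it heavy.
; The event graph holds only disabled placeholder events.
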(fn `UserConstructionScript`
  (bind _obsaclemeshes (`self.ObsacleMeshes`))
  (bind _obstaclematerials (`self.ObstacleMaterials`))
  (bind _staticmesh (`self.StaticMesh`))
  (`StaticMeshComponent.SetStaticMesh` (`self.StaticMesh`) (`|GetArrayItem` _obsaclemeshes (`KismetMathLibrary.RandomInteger` (`KismetArrayLibrary.Array_Length` _obsaclemeshes))))
  (`PrimitiveComponent.SetSimulatePhysics` (`self.StaticMesh`) true)
  (`PrimitiveComponent.SetMaterial` _staticmesh 0 (`|GetArrayItem` _obstaclematerials (`KismetMathLibrary.RandomInteger` (`KismetArrayLibrary.Array_Length` _obstaclematerials))))
  (`PrimitiveComponent.SetMassScale` _staticmesh "None" 100.0))