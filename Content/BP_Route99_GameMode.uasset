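; Game mode for an endless road driver, handling the paused main menu, game start, checkpoint score and game-over screen.
; InitiateGame lays initial straight tiles; SpawnRoadSection adds straights or occasional random sharp or gradual corners after a cooldown.
; Each piece spawns at the previous one's attach transform, with fuel or obstacles on a randomised real-time timer.
; Straights also get lamps on that timer, plus checkpoints at growing distance intervals.
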(event `self.ReceiveBeginPlay`
  (bind _returnvalue (`GameplayStatics.GetPlayerController` 0))
  (`GameplayStatics.SetGamePaused` true)
  (bind _returnvalue_2 (`|CreateWidget` "/Game/UI/BP_MainMenu.BP_MainMenu_C"))
  (set `PlayerController.bShowMouseCursor` true _returnvalue)
  (`WidgetBlueprintLibrary.SetInputMode_UIOnlyEx` _returnvalue _returnvalue_2)
  (`UserWidget.AddToViewport` _returnvalue_2 0))

(event `self.ReceiveTick`
  (params (DeltaSeconds :type "Float (single-precision)")))

(fn `AddFloorCornerL`
  (locals (CornerSection :type "/Game/Road/BP_Corner_L_Sharp Object Reference"))
  (bind _returnvalue (`|SpawnActorFromClass` "/Game/Road/BP_Corner_L_Sharp.BP_Corner_L_Sharp_C" (`self.Next Spawn Point`) "Undefined" "OverrideRootScale" null null))
  (bind _output_get (set `local.CornerSection` _returnvalue))
  (bind _returnvalue_2 (`/Game/Road/BP_Corner_L_Sharp.Get Attach Transform` _output_get))
  (set `self.Next Spawn Point` _returnvalue_2)
  (bind _spawn (`self.SpawnTimer`))
  (if _spawn
    (switch `int` (`KismetMathLibrary.RandomIntegerInRange` 0 1)
      (:`Default`
        (`/Game/Road/BP_Corner_L_Sharp.SpawnFuelPickup` (`local.CornerSection`) :!label _label))
      (:`0`
        (goto _label))
      (:`1`
        (`/Game/Road/BP_Corner_L_Sharp.SpawnObsticle` (`local.CornerSection`))))))

(fn `AddFloorCornerR`
  (locals (CornerSection :type "/Game/Road/BP_Corner_R_Sharp Object Reference"))
  (bind _returnvalue (`|SpawnActorFromClass` "/Game/Road/BP_Corner_R_Sharp.BP_Corner_R_Sharp_C" (`self.Next Spawn Point`) "Undefined" "OverrideRootScale" null null))
  (bind _output_get (set `local.CornerSection` _returnvalue))
  (bind _returnvalue_2 (`/Game/Road/BP_Corner_R_Sharp.Get Attach Transform` _output_get))
  (set `self.Next Spawn Point` _returnvalue_2)
  (bind _spawn (`self.SpawnTimer`))
  (if _spawn
    (switch `int` (`KismetMathLibrary.RandomIntegerInRange` 0 1)
      (:`Default`
        (`/Game/Road/BP_Corner_R_Sharp.SpawnFuelPickup` (`local.CornerSection`) :!label _label))
      (:`0`
        (goto _label))
      (:`1`
        (`/Game/Road/BP_Corner_R_Sharp.SpawnObsticle` (`local.CornerSection`))))))

(fn `AddFloorGradualCornerL`
  (locals (CornerSection :type "/Game/Road/BP_Corner_L_Gradual Object Reference"))
  (bind _returnvalue (`|SpawnActorFromClass` "/Game/Road/BP_Corner_L_Gradual.BP_Corner_L_Gradual_C" (`self.Next Spawn Point`) "Undefined" "OverrideRootScale" null null))
  (bind _asbp_corner_l_gradual (cast `/Game/Road/BP_Corner_L_Gradual` _returnvalue))
  (bind _output_get (set `local.CornerSection` _asbp_corner_l_gradual))
  (bind _returnvalue_2 (`/Game/Road/BP_Corner_L_Gradual.Get Attach Transform` _output_get))
  (set `self.Next Spawn Point` _returnvalue_2)
  (bind _spawn (`self.SpawnTimer`))
  (if _spawn
    (switch `int` (`KismetMathLibrary.RandomIntegerInRange` 0 1)
      (:`Default`
        (`/Game/Road/BP_Corner_L_Gradual.SpawnFuelPickup` (`local.CornerSection`) :!label _label))
      (:`0`
        (goto _label))
      (:`1`
        (`/Game/Road/BP_Corner_L_Gradual.SpawnObsticle` (`local.CornerSection`))))))

(fn `AddFloorGradualCornerR`
  (locals (CornerSection :type "/Game/Road/BP_Corner_R_Gradual Object Reference"))
  (bind _returnvalue (`|SpawnActorFromClass` "/Game/Road/BP_Corner_R_Gradual.BP_Corner_R_Gradual_C" (`self.Next Spawn Point`) "Undefined" "OverrideRootScale" null null))
  (bind _output_get (set `local.CornerSection` _returnvalue))
  (bind _returnvalue_2 (`/Game/Road/BP_Corner_R_Gradual.Get Attach Transform` _output_get))
  (set `self.Next Spawn Point` _returnvalue_2)
  (bind _spawn (`self.SpawnTimer`))
  (if _spawn
    (switch `int` (`KismetMathLibrary.RandomIntegerInRange` 0 1)
      (:`Default`
        (`/Game/Road/BP_Corner_R_Gradual.SpawnFuelPickup` (`local.CornerSection`) :!label _label))
      (:`0`
        (goto _label))
      (:`1`
        (`/Game/Road/BP_Corner_R_Gradual.SpawnObsticle` (`local.CornerSection`))))))

(fn `AddFloorTile`
  (locals (RoadSection :type "/Game/Road/BP_Road Object Reference"))
  (bind _returnvalue (`|SpawnActorFromClass` "/Game/Road/BP_Road.BP_Road_C" (`self.Next Spawn Point`) "Undefined" "OverrideRootScale" null null))
  (bind _asbp_road (cast `/Game/Road/BP_Road` _returnvalue))
  (bind _output_get (set `local.RoadSection` _asbp_road))
  (bind _returnvalue_2 (`/Game/Road/BP_Road.Get Attach Transform` _output_get))
  (set `self.Next Spawn Point` _returnvalue_2)
  (bind _spawn (`self.SpawnTimer`))
  (if _spawn
    (switch `int` (`KismetMathLibrary.RandomIntegerInRange` 0 1)
      (:`Default`
        (`/Game/Road/BP_Road.SpawnFuelPickup` (`local.RoadSection`) :!label _label))
      (:`0`
        (goto _label))
      (:`1`
        (`/Game/Road/BP_Road.SpawnObsticle` (`local.RoadSection`))))
    (`/Game/Road/BP_Road.SpawnLamp` (`local.RoadSection`)))
  (if (> (`self.CurrentLocation`) (`self.NextTimeout`))
    (`/Game/Road/BP_Road.SpawnCheckpoint` (`local.RoadSection`))
    (set `self.NextTimeout` (+ (`self.CurrentLocation`) (+ (`self.NextTimeout`) (/ (`self.NextTimeout`) 20))))))

(fn `GameOver`
  (bind _returnvalue (`GameplayStatics.GetPlayerController` 0))
  (bind _returnvalue_2 (`|CreateWidget` "/Game/UI/BP_GameOver.BP_GameOver_C"))
  (set `PlayerController.bShowMouseCursor` true _returnvalue)
  (`WidgetBlueprintLibrary.SetInputMode_UIOnlyEx` _returnvalue _returnvalue_2)
  (`UserWidget.AddToViewport` _returnvalue_2 0))

(fn `IncreaseCheckpointCount`
  (set `self.Score` (+ (`self.Score`) 1)))

(fn `InitiateGame`
  (locals (StartSpot :type "Actor Object Reference"))
  (`GameplayStatics.PlaySoundAtLocation` "/Game/Sound/chasing_speed.chasing_speed" (0.0 0.0 0.0) (struct) 1.0 1.0 0.0 null null null null)
  (for _ (range 20)
    (`self.AddFloorTile`)
    (`GameplayStatics.SetGamePaused` false)))

(fn `SetNextSpawnTime`
  (set `self.NextSpawn` (+ (`GameplayStatics.GetRealTimeSeconds`) (`KismetMathLibrary.RandomFloatInRange` (`self.SpawnFrequencyMin`) (`self.SpawnFrequencyMax`))))
  (return))

(fn `SpawnRoadSection`
  (bind _currentlocation (`self.CurrentLocation`))
  (bind _returnvalue (> (`self.LastCorner`) 10))
  (if _returnvalue
    (set `self.LastCorner` 0)
    (else
      (set `self.LastCorner` (+ (`self.LastCorner`) 1))))
  (if (and _returnvalue (> (`KismetMathLibrary.RandomFloatInRange` 0.0 100.0) 80.0))
    (if (>= (`KismetMathLibrary.RandomIntegerInRange` 0 100) 70)
      (if (`KismetMathLibrary.RandomBool`)
        (`self.AddFloorCornerL`)
        (else
          (`self.AddFloorCornerR`)))
      (elif (`KismetMathLibrary.RandomBool`)
        (`self.AddFloorGradualCornerL`)
        (else
          (`self.AddFloorGradualCornerR`))))
    (set `self.CurrentLocation` (+ _currentlocation 5))
    (else
      (`self.AddFloorTile`)
      (set `self.CurrentLocation` (+ _currentlocation 1)))))

(fn `SpawnTimer`
  (returns (Spawn :type Boolean))
  (if (<= (`self.NextSpawn`) 0.0)
    (`self.SetNextSpawnTime`))
  (bind _output_get (set `self.SpawnItem` (> (`GameplayStatics.GetRealTimeSeconds`) (`self.NextSpawn`))))
  (if _output_get
    (`self.SetNextSpawnTime`))
  (return (`self.SpawnItem`)))

(fn `UserConstructionScript`)