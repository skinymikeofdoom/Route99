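; BP_Corner_R_Sharp is a sharp right corner road tile for the Route 99 driving game's chain of spawned tiles.
; When a SportsCar_Pawn overlaps EndTrigger, it asks the game mode to add a floor tile, then destroys itself ten seconds later.
; GetAttachTransform exposes the AttachPoint transform, while fuel and obstacle functions add child actors at random points within PickupSpawnArea.
; Spline mesh construction code is present but disconnected.
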(event `self.EndTrigger.OnComponentBeginOverlap`
  (params (OverlappedComponent :type "PrimitiveComponent Object Reference") (OtherActor :type "Actor Object Reference") (OtherComp :type "PrimitiveComponent Object Reference") (OtherBodyIndex :type Integer) (bFromSweep :type Boolean) (SweepResult :type "HitResult Structure (by ref)"))
  (cast `/Game/VehicleTemplate/Blueprints/SportsCar/SportsCar_Pawn` OtherActor)
  (bind _asbp_route_99_game_mode (cast `/Game/BP_Route99_GameMode` (`GameplayStatics.GetGameMode`)))
  (`/Game/BP_Route99_GameMode.AddFloorTile` _asbp_route_99_game_mode)
  (`KismetSystemLibrary.Delay` 10.0)
  (`self.K2_DestroyActor`))

(fn `Get Attach Transform`
  (returns (ReturnValue :type "Transform Structure"))
  (return (`SceneComponent.K2_GetComponentToWorld` (`self.AttachPoint`))))

(fn `SpawnFuelPickup`
  (locals (GammeMode :type "/Game/BP_Route99_GameMode Object Reference"))
  (bind _pickup_spawn_area (`self.Pickup_Spawn_Area`))
  (`AddComponent|NODE_AddChildActorComponent-0` :`RelativeTransform` (`KismetMathLibrary.Conv_VectorToTransform` (`KismetMathLibrary.RandomPointInBoundingBox` (`SceneComponent.RelativeLocation` _pickup_spawn_area) (`BoxComponent.BoxExtent` _pickup_spawn_area)))))

(fn `SpawnObsticle`
  (bind _pickup_spawn_area (`self.Pickup_Spawn_Area`))
  (`AddComponent|NODE_AddChildActorComponent-1` :`RelativeTransform` (`KismetMathLibrary.Conv_VectorToTransform` (`KismetMathLibrary.RandomPointInBoundingBox` (`SceneComponent.RelativeLocation` _pickup_spawn_area) (`BoxComponent.BoxExtent` _pickup_spawn_area)))))

(fn `UserConstructionScript`)